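; Player character Blueprint that grants sprint and projectile attack abilities and prints debug readouts of credits and health.
; On BeginPlay it adds both action classes to its action component, then prints the credits read from MyPlayerState.
; The attribute component's health-changed event prints each new health value to screen.
; The MainHUD creation nodes are disconnected and never run, and the construction script is empty.
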(event OnHealthChanged(AttributeComp)
  (params (InstigatorActor :type Actor%20Object%20Reference) (OwningComp :type Attribute%20Component%20Object%20Reference) (NewHeawlth :type Float%20%28single-precision%29) (Delta :type Float%20%28single-precision%29))
  (Development|PrintString (Utilities|String|ToString(Float) NewHeawlth) true false "(R=1.000000,G=0.066792,B=0.582513,A=1.000000)"))

(event EventBeginPlay
  (bind _actioncomp (Variables|Default|GetActionComp))
  (Utilities|FlowControl|Sequence
    (:then_0
      (Class|ActionComponent|AddAction _actioncomp 0 "/Game/Actions/Action_SprintBP.Action_SprintBP_C"))
    (:then_1
      (Class|ActionComponent|AddAction _actioncomp 0 "/Game/Actions/Action_ProjectAttackBP.Action_ProjectAttackBP_C"))
    (:then_2
      (bind _asmy_player_state (Utilities|Casting|CastToMyPlayerState (Variables|Default|GetPlayerState))
        (:then
          (bind _returnvalue (Class|MyPlayerState|GetCredits _asmy_player_state))
          (Development|PrintString (Utilities|String|ToString(Float) _returnvalue) true true "(R=1.000000,G=0.000000,B=0.070174,A=1.000000)"))
        (:CastFailed
          (Development|PrintString "failed"))))))

(fn ConstructionScript)