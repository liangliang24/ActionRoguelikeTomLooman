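; Player controller Blueprint that sets up the main HUD and handles save and pause-menu hotkeys.
; On possess, a local controller adds the MainHUD widget to the viewport and switches to game-only input.
; L calls WriteSaveGame on MyGameModeBase and prints a confirmation.
; Escape or M creates a high Z-order pause menu widget, shows the cursor and switches to UI-only input, without actually pausing the game.
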(event EventPossess
  (params (PossessedPawn :type Pawn%20Object%20Reference))
  (if (Pawn|IsLocalController)
    (bind _returnvalue (UserInterface|CreateWidget "/Game/UI/MainHUD.MainHUD_C"))
    (UserInterface|Viewport|AddtoViewport _returnvalue 0)
    (Input|SetInputModeGameOnly self)))

(event Input|KeyboardEvents|L
  (params (Key :type Key%20Structure :default "None"))
  (:Pressed
    (bind _asmy_game_mode_base (Utilities|Casting|CastToMyGameModeBase (Game|GetGameMode)))
    (Class|MyGameModeBase|WriteSaveGame _asmy_game_mode_base)
    (Development|PrintString "Word Saved")))

(event Input|KeyboardEvents|Escape
  (params (Key :type Key%20Structure :default "None"))
  (:Pressed
    (bind _returnvalue (UserInterface|CreateWidget "/Game/UI/Menu/PauseMenu_Widget.PauseMenu_Widget_C"))
    (UserInterface|Viewport|AddtoViewport _returnvalue 100)
    (Variables|Default|SetbShowMouseCursor true)
    (Input|SetInputModeUIOnly self 0 "DoNotLock")))

(event Input|KeyboardEvents|M
  (params (Key :type Key%20Structure :default "None"))
  (:Pressed
    (bind _returnvalue (UserInterface|CreateWidget "/Game/UI/Menu/PauseMenu_Widget.PauseMenu_Widget_C"))
    (UserInterface|Viewport|AddtoViewport _returnvalue 100)
    (Variables|Default|SetbShowMouseCursor true)
    (Input|SetInputModeUIOnly self 0 "DoNotLock")))

(fn ConstructionScript)