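; Item chest actor whose Interact event only forwards to the parent implementation, while Tick prints the LidOpened state on screen in red for debugging.
; A disconnected leftover graph holds a key card gameplay tag check with empty branches and a FlipFlop-driven timeline that pitches the lid open or closed and activates particles once the animation finishes.
; None of that Blueprint lid logic runs.
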(event EventBeginPlay)

(event Collision|EventActorBeginOverlap
  (params (OtherActor :type Actor%20Object%20Reference)))

(event EventTick
  (params (DeltaSeconds :type Float%20%28single-precision%29))
  (Development|PrintString (Utilities|String|ToString(Boolean) (Variables|Default|GetbLidOpened)) true true "(R=1.000000,G=0.000000,B=0.000000,A=1.000000)" 0.0))

(event EventInteract
  (params (InstigatorPawn :type Pawn%20Object%20Reference))
  (|CallParentFunction InstigatorPawn))

(fn ConstructionScript)